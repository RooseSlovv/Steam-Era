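; BP_Protecter is a sphere actor that orbits a center actor, following it as it moves.
; Each tick it re-orthogonalizes the orbit axis against its radial offset using a double cross product, then rotates that offset by Speed scaled by delta time.
; It adds local yaw spin per frame, unscaled by delta time, while the center actor is valid.
; The construction script applies the sphere's material.
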(event `OrthogonalizeAxis`
  (bind _returnvalue (- (`self.K2_GetActorLocation`) (`self.Old Center Location`)))
  (set `self.Axis` (`KismetMathLibrary.Normal` (`KismetMathLibrary.Cross_VectorVector` _returnvalue (`KismetMathLibrary.Cross_VectorVector` (`self.Axis`) _returnvalue)))))

(event `self.ReceiveBeginPlay`
  (`|ExecutionSequence`
    (:`then_0`
      (bind _centoractor (`self.CentorActor`)
        (:`then`
          (set `self.Center Location` (`self.K2_GetActorLocation` _centoractor)))
        (:`else`)))
    (:`then_1`
      (set `self.Old Center Location` (`self.Center Location`)))))

(event `self.ReceiveTick`
  (params (DeltaSeconds :type "Float (single-precision)"))
  (`|ExecutionSequence`
    (:`then_0`
      (bind _centoractor (`self.CentorActor`)
        (:`then`
          (set `self.Center Location` (`self.K2_GetActorLocation` _centoractor))
          (`self.K2_AddActorLocalRotation` (`KismetMathLibrary.MakeRotator` 0.0 0.0 (`self.selfRotation`))))
        (:`else`)))
    (:`then_1`
      (`self.OrthogonalizeAxis`)
      (`self.K2_SetActorLocation` (+ (`KismetMathLibrary.RotateAngleAxis` (- (`self.K2_GetActorLocation`) (`self.Old Center Location`)) (* DeltaSeconds (`self.Speed`)) (`self.Axis`)) (`self.Center Location`)))
      (set `self.Old Center Location` (`self.Center Location`)))))

(fn `UserConstructionScript`
  (`PrimitiveComponent.SetMaterial` (`self.Sphere`) 0 (`self.Material_Instance`)))
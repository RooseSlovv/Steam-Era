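; BP_Icy is a player-driven laser actor that aims with the player camera and responds to the shoot input.
; It caches the platforming character on BeginPlay and copies that camera's world rotation onto its Icy component every tick.
; IA_Shoot sets InvertSystem on ACHandler while held and clears it on release or cancel, with debug prints.
; Controller lookup and ACExternal delegate linking are disconnected, and GatSocketLocation is an empty stub.
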(event `self.ReceiveBeginPlay`
  (bind _asbp_platforming_character (cast `/Game/Variant_Platforming/Blueprints/BP_PlatformingCharacter` (`GameplayStatics.GetPlayerCharacter` 0))))

(event `self.ReceiveTick`
  (params (DeltaSeconds :type "Float (single-precision)"))
  (bind (_returnvalue_roll _returnvalue_pitch _returnvalue_yaw) (`KismetMathLibrary.BreakRotator` (`SceneComponent.K2_GetComponentRotation` (`/Game/Variant_Platforming/Blueprints/BP_PlatformingCharacter.Camera` (stale `self.ReceiveBeginPlay` _asbp_platforming_character)))))
  (`SceneComponent.K2_SetWorldRotation` (`self.Icy`) (`KismetMathLibrary.MakeRotator` _returnvalue_roll _returnvalue_pitch _returnvalue_yaw) false false))

(event `EnhancedInput|/Game/Input/Actions/IA_Shoot`
  (params (ActionValue :type Boolean) (ElapsedSeconds :type "Float (double-precision)") (TriggeredSeconds :type "Float (double-precision)") (InputAction :type "InputAction Object Reference" :default "/Game/Input/Actions/IA_Shoot.IA_Shoot"))
  ;[1 1 1] Shoot Input
  (:`Started`
    ;;[0 0 0] Start Shooting Laser
    (set `/Game/Lasers/Blueprints/BuildingBlocks/AC_Handler.Invert System` true (`self.AC_Handler`))
    (`KismetSystemLibrary.PrintString` "Hello"))
  (:`Canceled`
    ;;[0 0 0] Stop Shooting Laser
    (set `/Game/Lasers/Blueprints/BuildingBlocks/AC_Handler.Invert System` false (`self.AC_Handler`) :!label _label)
    (`KismetSystemLibrary.PrintString` "Bye"))
  (:`Completed`
    (goto _label)))

(fn `GatSocketLocation`)

(fn `UserConstructionScript`)
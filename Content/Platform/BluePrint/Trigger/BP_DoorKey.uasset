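; BP_DoorKey is a pickup key actor for the platforming player character.
; It caches the player as a BP_PlatformingCharacter on BeginPlay and compares it against actors entering its Box trigger.
; On a match, PickupKey sets the character's DoorKey flag, plays a sound at its location and destroys itself.
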(event `self.ReceiveBeginPlay`
  (bind _asbp_platforming_character (cast `/Game/Variant_Platforming/Blueprints/BP_PlatformingCharacter` (`GameplayStatics.GetPlayerCharacter` 0)))
  (set `self.As BP Platforming Character` _asbp_platforming_character))

(event `PickupKey`
  (set `/Game/Variant_Platforming/Blueprints/BP_PlatformingCharacter.DoorKey` true (`self.As BP Platforming Character`))
  (`GameplayStatics.PlaySoundAtLocation` null (`self.K2_GetActorLocation`) (struct) 1.0 1.0 0.0 null null null null)
  (`self.K2_DestroyActor`))

(event `self.Box.OnComponentBeginOverlap`
  (params (OverlappedComponent :type "PrimitiveComponent Object Reference") (OtherActor :type "Actor Object Reference") (OtherComp :type "PrimitiveComponent Object Reference") (OtherBodyIndex :type Integer) (bFromSweep :type Boolean) (SweepResult :type "HitResult Structure (by ref)"))
  (if (== OtherActor (`self.As BP Platforming Character`))
    (`self.PickupKey`)))

(fn `UserConstructionScript`)
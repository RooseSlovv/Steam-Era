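; BP_IceSpawner is a platform spawner that repeatedly creates flattened actors, presumably ice going by its name, above its capsule.
; On BeginPlay, a loop spawns SpawnIndex copies of the configured class at the capsule's location raised by CapsuleHalfHeight.
; A Delay in the loop body feeds back into the loop, repeating the burst every few seconds.
; SpawnIce is empty, and the timer and capsule-sizing nodes never run.
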(event `SpawnIce`)

(event `self.ReceiveBeginPlay`
  (bind (_returnvalue_x _returnvalue_y _returnvalue_z) (`KismetMathLibrary.BreakVector` (`SceneComponent.K2_GetComponentLocation` (`self.Capsule`))))
  (for _ (range (`self.SpawnIndex`)) :!label _label
    (`|SpawnActorFromClass` (`self.SpawnActor`) (`KismetMathLibrary.MakeTransform` (`KismetMathLibrary.MakeVector` _returnvalue_x _returnvalue_y (+ _returnvalue_z (`self.Capsule Half Height`))) (struct) (1.0 1.0 0.3)) "Undefined" "MultiplyWithRoot" null null)
    (`KismetSystemLibrary.Delay` 7.0)
    (goto _label)))

(fn `UserConstructionScript`)
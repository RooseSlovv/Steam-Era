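; Platform obstacle Blueprint that moves four sticks vertically along Z in two opposed pairs, A/B and C/D.
; BeginPlay caches each stick's relative location, then one timeline drives A and B, and its update calls Play on a second timeline for C and D.
; In each pair, one stick adds the curve value and its partner the absolute difference from a fixed height.
; Disconnected leftover nodes hold an unused variant with doubled travel.
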(event `self.ReceiveBeginPlay`
  (bind (_alocation_x _alocation_y _alocation_z) (`KismetMathLibrary.BreakVector` (`self.ALocation`)))
  (bind (_blocation_x _blocation_y _blocation_z) (`KismetMathLibrary.BreakVector` (`self.BLocation`)))
  (bind (_clocation_x _clocation_y _clocation_z) (`KismetMathLibrary.BreakVector` (`self.CLocation`)))
  (bind (_dlocation_x _dlocation_y _dlocation_z) (`KismetMathLibrary.BreakVector` (`self.DLocation`)))
  (set `self.ALocation` (`SceneComponent.RelativeLocation` (`self.StickA`)))
  (set `self.BLocation` (`SceneComponent.RelativeLocation` (`self.StickB`)))
  (set `self.CLocation` (`SceneComponent.RelativeLocation` (`self.StickC`)))
  (set `self.DLocation` (`SceneComponent.RelativeLocation` (`self.StickD`)))
  (bind (_direction _up_down) (`Timeline|Timeline`)
    (:`Update`
      (`SceneComponent.K2_SetRelativeLocation` (`self.StickA`) (`KismetMathLibrary.MakeVector` _alocation_x _alocation_y (+ _alocation_z _up_down)) false false)
      (`SceneComponent.K2_SetRelativeLocation` (`self.StickB`) (`KismetMathLibrary.MakeVector` _blocation_x _blocation_y (+ _blocation_z (`KismetMathLibrary.Abs` (- _up_down 195.0)))) false false)
      (bind (_direction_2 _up_down_2) (`Timeline|Timeline_0`)
        (:`Update`
          (`SceneComponent.K2_SetRelativeLocation` (`self.StickC`) (`KismetMathLibrary.MakeVector` _clocation_x _clocation_y (+ _clocation_z _up_down_2)) false false)
          (`SceneComponent.K2_SetRelativeLocation` (`self.StickD`) (`KismetMathLibrary.MakeVector` _dlocation_x _dlocation_y (+ _dlocation_z (`KismetMathLibrary.Abs` (- _up_down_2 195.0)))) false false))))))

(fn `UserConstructionScript`)
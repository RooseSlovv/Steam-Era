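; Conveyor belt platform that starts stopped, with its CustomTimeDilation set to zero on BeginPlay.
; Tick offsets every actor overlapping the Box along the Arrow's forward vector by Speed times DeltaSeconds, without sweeping.
; The zero dilation scales the actor's delta time to zero, so the belt moves nothing, and this Blueprint never restores it.
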(event `self.ReceiveBeginPlay`
  (set `self.CustomTimeDilation` 0.0))

(event `self.ReceiveTick`
  (params (DeltaSeconds :type "Float (single-precision)"))
  (for _array_element (`PrimitiveComponent.GetOverlappingActors` (`self.Box`) null)
    (`self.K2_AddActorWorldOffset` _array_element (* (* DeltaSeconds (`self.Speed`)) (`SceneComponent.GetForwardVector` (`self.Arrow`))) false false)))

(fn `UserConstructionScript`)
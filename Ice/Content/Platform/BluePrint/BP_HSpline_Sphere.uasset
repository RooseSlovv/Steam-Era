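; Spline-path actor that moves its Cylinder component along a spline at a set speed, apparently as a moving platform.
; The construction script lays a spline mesh between each pair of consecutive spline points to show the path.
; Tick accumulates distance and places the Cylinder there in local space, following only the spline's yaw with a quarter-turn offset.
; With Loop enabled, the distance snaps back to the start after passing the spline's end.
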(event `self.ReceiveTick`
  (params (DeltaSeconds :type "Float (single-precision)"))
  (bind _returnvalue (`SplineComponent.GetTransformAtDistanceAlongSpline` (`self.Spline`) (`self.Distance`) "Local" false))
  (set `self.Distance` (+ (* DeltaSeconds (`self.Speed`)) (`self.Distance`)))
  (`SceneComponent.K2_SetRelativeTransform` (`self.Cylinder`) (`KismetMathLibrary.MakeTransform` (.location _returnvalue) (`KismetMathLibrary.MakeRotator` 0.0 0.0 (+ (.yaw (.rotation _returnvalue)) -90.0)) (`SceneComponent.RelativeScale3D` (`self.Cylinder`))) false false)
  (if (`self.loop`)
    (if (> (`self.Distance`) (`SplineComponent.GetSplineLength` (`self.Spline`)))
      (set `self.Distance` 0.0))))

(fn `UserConstructionScript`
  (bind _spline (`self.Spline`))
  (for _index (range (+ (- (`SplineComponent.GetNumberOfSplinePoints` (`self.Spline`)) 2) 1))
    (bind _returnvalue (`AddComponent|NODE_AddSplineMeshComponent-1`))
    (`self.K2_AttachToComponent` (`self.DefaultSceneRoot`) "None" "KeepRelative" "KeepRelative" "KeepRelative")
    (`SplineMeshComponent.SetForwardAxis` _returnvalue "X" true)
    (bind (_location _tangent) (`SplineComponent.GetLocationAndTangentAtSplinePoint` _spline _index "Local"))
    (bind (_location_2 _tangent_2) (`SplineComponent.GetLocationAndTangentAtSplinePoint` _spline (+ _index 1) "Local"))
    (`SplineMeshComponent.SetStartAndEnd` _returnvalue _location _tangent _location_2 _tangent_2 true)))
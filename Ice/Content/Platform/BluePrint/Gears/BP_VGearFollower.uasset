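; BP_VGearFollower is a platforming gear hazard that follows another actor's rotation and knocks the player away on contact.
; Each tick it reads the yaw of the referenced Force actor and applies it to its own rotation.
; Overlapping any of its three capsules launches a BP_PlatformingCharacter with the same fixed horizontal X and Y velocity, independent of the gear's orientation.
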(event `self.ReceiveTick`
  (params (DeltaSeconds :type "Float (single-precision)"))
  (bind (_returnvalue_roll _returnvalue_pitch _returnvalue_yaw) (`KismetMathLibrary.BreakRotator` (`self.K2_GetActorRotation` (`self.Force`))))
  (`self.K2_SetActorRotation` (`KismetMathLibrary.MakeRotator` 0.0 0.0 _returnvalue_yaw)))

(event `self.Capsule01.OnComponentBeginOverlap`
  (params (OverlappedComponent :type "PrimitiveComponent Object Reference") (OtherActor :type "Actor Object Reference") (OtherComp :type "PrimitiveComponent Object Reference") (OtherBodyIndex :type Integer) (bFromSweep :type Boolean) (SweepResult :type "HitResult Structure (by ref)"))
  (bind _asbp_platforming_character (cast `/Game/Variant_Platforming/Blueprints/BP_PlatformingCharacter` OtherActor))
  (`Character.LaunchCharacter` _asbp_platforming_character (700.0 700.0 0.0) false false))

(event `self.Capsule02.OnComponentBeginOverlap`
  (params (OverlappedComponent :type "PrimitiveComponent Object Reference") (OtherActor :type "Actor Object Reference") (OtherComp :type "PrimitiveComponent Object Reference") (OtherBodyIndex :type Integer) (bFromSweep :type Boolean) (SweepResult :type "HitResult Structure (by ref)"))
  (bind _asbp_platforming_character (cast `/Game/Variant_Platforming/Blueprints/BP_PlatformingCharacter` OtherActor))
  (`Character.LaunchCharacter` _asbp_platforming_character (700.0 700.0 0.0) false false))

(event `self.Capsule03.OnComponentBeginOverlap`
  (params (OverlappedComponent :type "PrimitiveComponent Object Reference") (OtherActor :type "Actor Object Reference") (OtherComp :type "PrimitiveComponent Object Reference") (OtherBodyIndex :type Integer) (bFromSweep :type Boolean) (SweepResult :type "HitResult Structure (by ref)"))
  (bind _asbp_platforming_character (cast `/Game/Variant_Platforming/Blueprints/BP_PlatformingCharacter` OtherActor))
  (`Character.LaunchCharacter` _asbp_platforming_character (700.0 700.0 0.0) false false))

(fn `UserConstructionScript`)
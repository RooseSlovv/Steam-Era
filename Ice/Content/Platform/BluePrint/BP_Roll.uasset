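; BP_Roll is a rotating wooden stick obstacle that knocks the platforming character away, with a Death variant that shows thorns.
; Tick spins the stick body by a fixed step each frame, independent of delta time.
; When Death is off, overlapping the capsule applies a strong impulse along the Arrow's forward vector.
; The construction script toggles thorn visibility from Death; this graph applies no push or damage in that mode.
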(event `self.ReceiveTick`
  (params (DeltaSeconds :type "Float (single-precision)"))
  (`SceneComponent.K2_AddRelativeRotation` (`self.SM_WoodStickBody`) (struct :`Yaw` 5.0) false false))

(event `self.Capsule.OnComponentBeginOverlap`
  (params (OverlappedComponent :type "PrimitiveComponent Object Reference") (OtherActor :type "Actor Object Reference") (OtherComp :type "PrimitiveComponent Object Reference") (OtherBodyIndex :type Integer) (bFromSweep :type Boolean) (SweepResult :type "HitResult Structure (by ref)"))
  (bind _asbp_platforming_character (cast `/Game/Variant_Platforming/Blueprints/BP_PlatformingCharacter` OtherActor))
  (if (not (`self.Death`))
    (`CharacterMovementComponent.AddImpulse` (`Character.CharacterMovement` _asbp_platforming_character) (* (`SceneComponent.GetForwardVector` (`self.Arrow`)) 70000.0) false)))

(fn `UserConstructionScript`
  (if (`self.Death`)
    (`SceneComponent.SetVisibility` (`self.SM_WoodStickThorm`) true false)
    (else
      (`SceneComponent.SetVisibility` (`self.SM_WoodStickThorm`) false false))))
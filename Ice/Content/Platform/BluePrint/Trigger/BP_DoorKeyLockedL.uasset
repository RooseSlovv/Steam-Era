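; A key-locked door that slides open along X when the platforming player character overlaps its collision while holding the door key.
; BeginPlay caches the player character, and the overlap checks that reference and its DoorKey flag, firing through a DoOnce to start the opening and play a sound.
; The DoorOpen timeline sets the mesh's relative location from its current world location plus the track's X each update, so the offset is reapplied to a moving base.
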(event `self.ReceiveBeginPlay`
  (bind _asbp_platforming_character (cast `/Game/Variant_Platforming/Blueprints/BP_PlatformingCharacter` (`GameplayStatics.GetPlayerCharacter` 0)))
  (set `self.As BP Platforming Character` _asbp_platforming_character))

(event `OpenDoor`
  (bind _sm_door (`self.SM_Door`))
  (bind (_returnvalue_x _returnvalue_y _returnvalue_z) (`KismetMathLibrary.BreakVector` (`SceneComponent.K2_GetComponentLocation` _sm_door)))
  (bind (_direction _newtrack_0) (`Timeline|DoorOpen`)
    (:`Update`
      (`SceneComponent.K2_SetRelativeLocation` _sm_door (`KismetMathLibrary.MakeVector` (+ _returnvalue_x (.x _newtrack_0)) _returnvalue_y _returnvalue_z) false false))))

(event `self.Col_Door.OnComponentBeginOverlap`
  (params (OverlappedComponent :type "PrimitiveComponent Object Reference") (OtherActor :type "Actor Object Reference") (OtherComp :type "PrimitiveComponent Object Reference") (OtherBodyIndex :type Integer) (bFromSweep :type Boolean) (SweepResult :type "HitResult Structure (by ref)"))
  (bind _as_bp_platforming_character (`self.As BP Platforming Character`))
  (if (== OtherActor _as_bp_platforming_character)
    (if (== (`/Game/Variant_Platforming/Blueprints/BP_PlatformingCharacter.DoorKey` _as_bp_platforming_character) true)
      (`/Engine/EditorBlueprintResources/StandardMacros.DoOnce` false
        (:`Completed`
          (`self.OpenDoor`)
          (`GameplayStatics.PlaySoundAtLocation` null (`self.K2_GetActorLocation`) (struct) 1.0 1.0 0.0 null null null null))))))

(fn `UserConstructionScript`)
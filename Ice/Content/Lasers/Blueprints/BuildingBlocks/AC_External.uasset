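; Actor component that links its owner to the laser system's AC_Handler components on target actors, for things like buttons and doors.
; With InvertControl it registers with each handler and drives it through External Activate/Deactivate events, as a button activates a laser spawn.
; Otherwise it listens to the handlers, tracking states in a map to activate only when all are active and deactivate when any drops, forwarding update alpha.
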(event `self.ReceiveBeginPlay`
  ;[1 1 1] Link the delegates and dispatched events if there is a target actor
  (if (`KismetArrayLibrary.Array_IsNotEmpty` (`self.TargetActors`))
    (`self.LinkDelegates`)))

(event `LinkDelegates`
  (if (`self.InvertControl`)
    ;[1 1 1] Check that the target actor is valid and does have a Handler component
    (for _array_element (`self.TargetActors`)
      (bind _returnvalue (`Actor.GetComponentByClass` _array_element "/Game/Lasers/Blueprints/BuildingBlocks/AC_Handler.AC_Handler_C"))
      (`/Engine/EditorBlueprintResources/StandardMacros.IsValid` _returnvalue
        (:`Is Valid`
          ;[1 1 1] Bind the activate and deactivate of this actor to the functions within the target handler
          (`KismetArrayLibrary.Array_AddUnique` (`/Game/Lasers/Blueprints/BuildingBlocks/AC_Handler.LinkedExternalComps` _returnvalue) self)
          (add `self.ExternalActivate` (`|CreateDelegate` _returnvalue :!event `ForceActivation`))
          (add `self.ExternalDeactivate` (`|CreateDelegate` _returnvalue :!event `ForceDeactivation`)))))
    (else
      (for _array_element_2 (`self.TargetActors`)
        (bind _returnvalue_2 (`Actor.GetComponentByClass` _array_element_2 "/Game/Lasers/Blueprints/BuildingBlocks/AC_Handler.AC_Handler_C"))
        (`/Engine/EditorBlueprintResources/StandardMacros.IsValid` _returnvalue_2
          (:`Is Valid`
            ;[1 1 1] Bind the events of the target handler to the functions of this component
            (`BlueprintMapLibrary.Map_Add` (`self.NecessaryActors`) _returnvalue_2 (`/Game/Lasers/Blueprints/BuildingBlocks/AC_Handler.Invert System` _returnvalue_2))
            (add `/Game/Lasers/Blueprints/BuildingBlocks/AC_Handler.ActivateHandler` _returnvalue_2 (`|CreateDelegate` :!event `Activate This`))
            (add `/Game/Lasers/Blueprints/BuildingBlocks/AC_Handler.DeactivateHandler` _returnvalue_2 (`|CreateDelegate` :!event `Deactivate This`))
            (add `/Game/Lasers/Blueprints/BuildingBlocks/AC_Handler.UpdateHandler` _returnvalue_2 (`|CreateDelegate` :!event `Update This`))))))))

(fn `Activate This`
  (params (Instigator :type "/Game/Lasers/Blueprints/BuildingBlocks/AC_Handler Object Reference"))
  (if (`self.InvertControl`)
    ;[1 1 1] Used in cases like a button to activate a laser spawn
    (set `self.IsCompActivated` true)
    (`self.ExternalActivate` (`self.ApplyConditions`))
    (else
      ;[1 1 1] Used in cases like Doors
      (`|ExecutionSequence`
        (:`then_0`
          (`BlueprintMapLibrary.Map_Add` (`self.NecessaryActors`) (`local.Instigator`) true))
        (:`then_1`
          (if (`self.AllActorsActive`)
            (`self.ExternalActivate` (`self.ApplyConditions`))))))))

(fn `AllActorsActive`
  (returns (OutputPin :type Boolean))
  ;[1 1 1] Loop through the necessary actors to see if any of them are false.
  (bind _keys (`BlueprintMapLibrary.Map_Keys` (`self.NecessaryActors`)))
  (for _array_element _keys
    (if (not (`BlueprintMapLibrary.Map_Find` (`self.NecessaryActors`) _array_element))
      (return false)))
  (return true))

(fn `Deactivate This`
  (params (Instigator :type "/Game/Lasers/Blueprints/BuildingBlocks/AC_Handler Object Reference"))
  (if (`self.InvertControl`)
    ;[1 1 1] Used in cases like a button to activate a laser spawn
    (set `self.IsCompActivated` false)
    (`self.ExternalDeactivate` (`self.ApplyConditions`))
    (else
      ;[1 1 1] Used in cases like Doors
      (`BlueprintMapLibrary.Map_Add` (`self.NecessaryActors`) (`local.Instigator`))
      (`self.ExternalDeactivate` (`self.ApplyConditions`)))))

(fn `Update This`
  (params (Alpha :type "Float (double-precision)"))
  (`self.ExternalUpdate` Alpha))
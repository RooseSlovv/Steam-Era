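; Laser building-block component that makes its owning actor bounce incoming lasers by spawning a reflected emitter for each one.
; Start, update and stop hit events spawn, move or destroy an SC_Emitter at the mirrored impact transform, tracked per input laser in EmitterBounceMap.
; Emitters optionally inherit the incoming laser's color, and forced activation or deactivation replays hits from the owning AC_Handler's filtered lasers.
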(event `self.ReceiveBeginPlay`
  (bind _returnvalue (`Actor.GetComponentByClass` (`self.GetOwner`) "/Game/Lasers/Blueprints/BuildingBlocks/AC_Handler.AC_Handler_C"))
  ;[1 1 1] Get the handler that is controlling this component
  (`/Engine/EditorBlueprintResources/StandardMacros.IsValid` _returnvalue
    (:`Is Valid`
      (set `self.OwningHandler` _returnvalue))))

(event `/Game/Lasers/Blueprints/BuildingBlocks/BPI_Lasers.Laser Start Hitting`
  (params (Input :type "/Game/Lasers/Blueprints/BuildingBlocks/A_Laser Object Reference") (`Hit Info` :type "HitResult Structure"))
  ;[1 1 1] Start Hitting Event
  (`/Engine/EditorBlueprintResources/StandardMacros.IsValid` Input
    (:`Is Valid`
      (if (not (`BlueprintMapLibrary.Map_Contains` (`self.EmitterBounceMap`) Input))
        (`self.SpawnLaser` Input `Hit Info`)))))

(event `/Game/Lasers/Blueprints/BuildingBlocks/BPI_Lasers.Laser Stop Hitting`
  (params (Input :type "/Game/Lasers/Blueprints/BuildingBlocks/A_Laser Object Reference"))
  ;[1 1 1] Stop Hitting Event
  (`self.RemoveLaser` Input))

(event `/Game/Lasers/Blueprints/BuildingBlocks/BPI_Lasers.Laser Update Hitting`
  (params (Input :type "/Game/Lasers/Blueprints/BuildingBlocks/A_Laser Object Reference") (`Hit Info` :type "HitResult Structure"))
  (bind (_location _rotation) (`self.Mirror Location Rotation` `Hit Info`))
  (bind (_value _returnvalue) (`BlueprintMapLibrary.Map_Find` (`self.EmitterBounceMap`) Input))
  ;[1 1 1] Update Hitting Laser
  (if _returnvalue
    (`SceneComponent.K2_SetWorldLocationAndRotation` _value _location _rotation false false)))

(event `/Game/Lasers/Blueprints/BuildingBlocks/BPI_Lasers.Intermediate Change`
  (params (Modified :type "/Game/Lasers/Blueprints/BuildingBlocks/A_Laser Object Reference"))
  ;[1 1 1] Intermediate Change Event
  ;;[0 0 0] Update the SC_Emitters color
  (bind _values (`BlueprintMapLibrary.Map_Values` (`self.EmitterBounceMap`)))
  (for _array_element _values
    (`/Game/Lasers/Blueprints/BuildingBlocks/SC_Emitter.Set Laser Color` _array_element)))

(event `/Game/Lasers/Blueprints/BuildingBlocks/BPI_Lasers.ForceActivation`
  (params (ApplyConditions :type Boolean))
  ;[1 1 1] Force Activation Event
  (for _array_element (`/Game/Lasers/Blueprints/BuildingBlocks/AC_Handler.FilteredLasers` (`self.OwningHandler`))
    (bind (_value _returnvalue) (`/Game/Lasers/Blueprints/BuildingBlocks/A_Laser.GetHitByHandler` _array_element (`self.OwningHandler`)))
    ;;[0 0 0] Needs to use the lasers hit information to re-activate the laser (can't force activate a bounce with no lasers)
    (if _returnvalue
      (`self.Laser Start Hitting` _array_element _value))))

(event `/Game/Lasers/Blueprints/BuildingBlocks/BPI_Lasers.ForceDeactivation`
  (params (ApplyConditions :type Boolean))
  ;[1 1 1] Force Deactivation Event
  (for _array_element (`/Game/Lasers/Blueprints/BuildingBlocks/AC_Handler.FilteredLasers` (`self.OwningHandler`))
    (`self.Laser Stop Hitting` _array_element)))

(fn `RemoveLaser`
  (params (InputPin :type "/Game/Lasers/Blueprints/BuildingBlocks/A_Laser Object Reference"))
  (locals (`L-RemoveItem` :type "/Game/Lasers/Blueprints/BuildingBlocks/SC_Emitter Object Reference"))
  (bind (_value _returnvalue) (`BlueprintMapLibrary.Map_Find` (`self.EmitterBounceMap`) (`local.InputPin`)))
  (if _returnvalue
    (bind _output_get (set `local.L-RemoveItem` _value))
    (`/Game/Lasers/Blueprints/BuildingBlocks/SC_Emitter.ForceDeactivation` _output_get false) ; Deactivate the emitter (remove the laser\nand deactivate subsequent targets)
    (`/Game/Lasers/Blueprints/BuildingBlocks/SC_Emitter.DestroySelf` (`local.L-RemoveItem`)) ; Destroy the SC_Emitter\ncomponent
    (`BlueprintMapLibrary.Map_Remove` (`self.EmitterBounceMap`) (`local.InputPin`))))

(fn `SpawnLaser`
  (params (`Laser In` :type "/Game/Lasers/Blueprints/BuildingBlocks/A_Laser Object Reference") (`Hit Info` :type "HitResult Structure"))
  (bind _returnvalue (`Actor.GetTransform` (`self.GetOwner`)))
  (bind (_location _rotation) (`self.Mirror Location Rotation` (`local.Hit Info`)))
  ;[1 1 1] Spawn Emitter component and attach it to the relected location & rotation
  (bind _returnvalue_2 (`|AddComponentByClass` (`self.GetOwner`) "/Game/Lasers/Blueprints/BuildingBlocks/SC_Emitter.SC_Emitter_C" false (`KismetMathLibrary.MakeTransform` (`KismetMathLibrary.InverseTransformLocation` _returnvalue _location) (`KismetMathLibrary.InverseTransformRotation` _returnvalue _rotation))))
  (`BlueprintMapLibrary.Map_Add` (`self.EmitterBounceMap`) (`local.Laser In`) _returnvalue_2) ; Store the laser that hit & the SC_Emitter\nthat was spawned
  ;[1 1 1] Should the lasers use the color that spawned them or use the handler rules (First Laser Hit, merged...)
  (if (`self.UseBounceColor`)
    (set `/Game/Lasers/Blueprints/BuildingBlocks/SC_Emitter.Override Color` (`/Game/Lasers/Blueprints/BuildingBlocks/A_Laser.ColorOverride` (`local.Laser In`)) _returnvalue_2)
    (set `/Game/Lasers/Blueprints/BuildingBlocks/SC_Emitter.UseOverride` true _returnvalue_2))
  (`/Game/Lasers/Blueprints/BuildingBlocks/SC_Emitter.Set Laser Color` _returnvalue_2)
  (`/Game/Lasers/Blueprints/BuildingBlocks/SC_Emitter.Activate Laser` _returnvalue_2))